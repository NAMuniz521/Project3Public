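; Pl_PowerUp_03 is a spinning platformer pickup that opens a gate, reveals a key and raises a platform.
; Any actor overlap destroys the linked gate, hides the pickup and unhides the key.
; A timeline then lerps the platform holder from its current location by an offset vector, and the pickup destroys itself when the rise finishes.
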(event `self.ReceiveTick`
  (params (DeltaSeconds :type "Float (single-precision)"))
  (`self.K2_AddActorLocalRotation` (struct :`Yaw` 5.0)))

(event `self.ReceiveActorBeginOverlap`
  (params (OtherActor :type "Actor Object Reference"))
  (`self.K2_DestroyActor` (`self.GateToOpen`))
  (`self.SetActorHiddenInGame` true)
  (`self.SetActorHiddenInGame` (`self.Key`) false)
  (bind _output_get (set `self.StartingPosition` (`self.K2_GetActorLocation` (`self.RisingPlatformHolder`))))
  (set `self.EndingPosition` (+ _output_get (`self.AddVector`)))
  (bind (_direction _up) (`Timeline|RaisePlatform` :!via `PlayFromStart`)
    (:`Update`
      (`self.K2_SetActorLocation` (`self.RisingPlatformHolder`) (`KismetMathLibrary.VLerp` (`self.StartingPosition`) (`self.EndingPosition`) _up) false false))
    (:`Finished`
      (`self.K2_DestroyActor`))))

(fn `UserConstructionScript`)